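; Dialogue NPC character that wanders the navmesh at a randomized walk speed and can talk to the player.
; A looping AI MoveTo picks random reachable points, pausing briefly between moves, while box overlap flags the ThirdPersonCharacter as near the AI.
; TalkEvent stops movement, turns the mesh toward the player, feeds DialogSequence to HUD widgets and plays the line's sound.
; Leaving the box mid-talk hides the text and restores speed and rotation.
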(event `self.ReceiveBeginPlay`
  ;[1 1 1] Walking Logic
  ;;[1 1 1] Give the AI a random walking speed
  (bind _output_get (set `self.Walk_Speed` (`KismetMathLibrary.RandomFloatInRange` 100.0 45.0)))
  (set `CharacterMovementComponent.MaxWalkSpeed` _output_get (`self.CharacterMovement`))
  (`self.WalkEvent`))

(event `WalkEvent`
  ;[1 1 1] Walking Logic
  ;;[1 1 1] Wandering Behavior for AI
  (if (not (`self.Walking`))
    (`|AIMoveTo` self (`NavigationSystem.K2_GetRandomLocationInNavigableRadius` (`self.K2_GetActorLocation`) (`self.Walk Radius`))
      (:`then`
        (set `self.Walking` true))
      (:`OnSuccess`
        (`KismetSystemLibrary.Delay` (`KismetMathLibrary.RandomFloatInRange` 1.0 5.0) :!label _label)
        (set `self.Walking` false)
        (`self.WalkEvent`))
      (:`OnFail`
        (goto _label)))))

(event `Talk Event`
  (bind _hudwidget (`self.HudWidget`))
  (bind _sound (`self.Sound`))
  (bind _speachindex (`/Game/Blueprints/HUD.SpeachIndex` _hudwidget))
  ;[1 1 1] Talk Event for the AI Character
  (set `self.Is Talking` true)
  (set `CharacterMovementComponent.MaxWalkSpeed` 0.0 (`self.CharacterMovement`))
  ;;[1 1 1] Set the rotation it currently is at before rotating it toward the player
  (set `self.Rotation` (`SceneComponent.K2_GetComponentRotation` (`self.Mesh`)))
  (`SceneComponent.K2_SetWorldRotation` (`self.Mesh`) (`KismetMathLibrary.MakeRotator` (.roll (`KismetMathLibrary.FindLookAtRotation` (`self.K2_GetActorLocation` self) (`self.K2_GetActorLocation` (`GameplayStatics.GetPlayerCharacter` 0)))) 0.0 (- (.yaw (`KismetMathLibrary.FindLookAtRotation` (`self.K2_GetActorLocation` self) (`self.K2_GetActorLocation` (`GameplayStatics.GetPlayerCharacter` 0)))) 90.0)) false false)
  (bind _foundwidgets (`WidgetBlueprintLibrary.GetAllWidgetsOfClass` "/Game/Blueprints/HUD.HUD_C"))
  (for _array_element _foundwidgets
    (bind _output_get (set `self.HudWidget` _array_element))
    ;;[1 1 1] Setting the Dialog
    (set `/Game/Blueprints/HUD.TurnOnTextBox` true _output_get)
    (set `/Game/Blueprints/HUD.Speech` (`self.DialogSequence`) _hudwidget)
    ;;[1 1 1] If there is a sound for the dialog play it else don't
    (if (not (> _speachindex (`KismetArrayLibrary.Array_Length` _sound)))
      (`GameplayStatics.PlaySoundAtLocation` (`|GetArrayItem` _sound _speachindex) (`SceneComponent.K2_GetComponentLocation` (`self.CapsuleComponent`))))))

(event `self.Box.OnComponentBeginOverlap`
  (params (OverlappedComponent :type "PrimitiveComponent Object Reference") (OtherActor :type "Actor Object Reference") (OtherComp :type "PrimitiveComponent Object Reference") (OtherBodyIndex :type Integer) (bFromSweep :type Boolean) (SweepResult :type "HitResult Structure (by ref)"))
  ;[1 1 1] Determine if the character is overlapping with the Box Collision on the AI
  (bind _asthird_person_character (cast `/Game/ThirdPersonCPP/Blueprints/ThirdPersonCharacter` OtherActor))
  (set `/Game/ThirdPersonCPP/Blueprints/ThirdPersonCharacter.AI Overlap` true _asthird_person_character))

(event `self.Box.OnComponentEndOverlap`
  (params (OverlappedComponent :type "PrimitiveComponent Object Reference") (OtherActor :type "Actor Object Reference") (OtherComp :type "PrimitiveComponent Object Reference") (OtherBodyIndex :type Integer))
  ;[1 1 1] Determine if the character is overlapping with the Box Collision on the AI
  (if (`self.Is Talking`)
    (bind _asthird_person_character (cast `/Game/ThirdPersonCPP/Blueprints/ThirdPersonCharacter` OtherActor))
    (set `/Game/ThirdPersonCPP/Blueprints/ThirdPersonCharacter.AI Overlap` false _asthird_person_character)
    (set `self.Is Talking` false)
    ;;[1 1 1] Return to normal wandering behavior and set dialogue to empty
    (set `CharacterMovementComponent.MaxWalkSpeed` (`self.Walk_Speed`) (`self.CharacterMovement`))
    (bind _foundwidgets (`WidgetBlueprintLibrary.GetAllWidgetsOfClass` "/Game/Blueprints/HUD.HUD_C"))
    (for _array_element _foundwidgets
      (set `/Game/Blueprints/HUD.TurnOnTextBox` false _array_element)
      ;;[1 1 1] Set the rotation back to what it was before talking
      (`SceneComponent.K2_SetWorldRotation` (`self.Mesh`) (`self.Rotation`) false false))))

(fn `UserConstructionScript`)