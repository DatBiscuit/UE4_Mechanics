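; Test actor that toggles ItemsToHide when a ThirdPersonCharacter enters or leaves its box trigger.
; Begin and end overlap share one path, which calls ToggleItem and sets a text render to On or Off from the resulting visibility.
; The text starts at Off on BeginPlay.
; After switching to On, a Delay loop polls the overlap but performs no other action.
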(event `self.ReceiveBeginPlay`
  (`TextRenderComponent.K2_SetText` (`self.TextRender`) (`self.Off`)))

(event `self.Box.OnComponentBeginOverlap`
  (params (OverlappedComponent :type "PrimitiveComponent Object Reference") (OtherActor :type "Actor Object Reference") (OtherComp :type "PrimitiveComponent Object Reference") (OtherBodyIndex :type Integer) (bFromSweep :type Boolean) (SweepResult :type "HitResult Structure (by ref)"))
  (bind _asthird_person_character (cast `/Game/ThirdPersonCPP/Blueprints/ThirdPersonCharacter` OtherActor))
  (set `self.Character` _asthird_person_character :!label _label)
  (`/Game/Blueprints/ToggleItem/ToggleItem.ToggleItem` (`self.ToggleItem`) (`self.Items to Hide`))
  (if (`SceneComponent.bVisible` (`self.Items to Hide`))
    (`TextRenderComponent.K2_SetText` (`self.TextRender`) (`self.On`))
    (if (`PrimitiveComponent.IsOverlappingActor` (`self.Box`) (`self.Character`)) :!label _label_2
      (`KismetSystemLibrary.Delay` 0.1)
      (goto _label_2))
    (else
      (`TextRenderComponent.K2_SetText` (`self.TextRender`) (`self.Off`)))))

(event `self.Box.OnComponentEndOverlap`
  (params (OverlappedComponent :type "PrimitiveComponent Object Reference") (OtherActor :type "Actor Object Reference") (OtherComp :type "PrimitiveComponent Object Reference") (OtherBodyIndex :type Integer))
  (cast `/Game/ThirdPersonCPP/Blueprints/ThirdPersonCharacter` OtherActor)
  (goto _label))

(fn `UserConstructionScript`)