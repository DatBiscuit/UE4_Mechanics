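; Actor component that shows or hides the player's minimap widget on the HUD, toggling it on at BeginPlay.
; ToggleMiniMap removes and clears an existing Minimap widget, or creates a new one otherwise.
; A new widget is added to the HudCanvas of MyPlayerController's HUD widget, auto-sized and anchored to the top-right corner at the Position offset.
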(event `self.ReceiveBeginPlay`
  (`self.ToggleMiniMap`))

(fn `ToggleMiniMap`
  (`self.Minimap`
    (:`then`
      (`Widget.RemoveFromParent` (`self.Minimap`))
      (set `self.Minimap` null))
    (:`else`
      (bind _returnvalue (`|CreateWidget` "/Game/Blueprints/Minimap.Minimap_C"))
      (set `self.Minimap` _returnvalue)
      (bind _asmy_player_controller (cast `/Game/Blueprints/MyPlayerController` (`GameplayStatics.GetPlayerController` 0)))
      (bind _returnvalue_2 (`CanvasPanel.AddChildToCanvas` (`/Game/Blueprints/HUD.HudCanvas` (`/Game/Blueprints/MyPlayerController.Hud Widget` _asmy_player_controller)) (`self.Minimap`)))
      (`CanvasPanelSlot.SetAutoSize` _returnvalue_2 true)
      (`CanvasPanelSlot.SetAlignment` _returnvalue_2 (1.0 0.0))
      (`CanvasPanelSlot.SetAnchors` _returnvalue_2 (make `Anchors` (1.0 0.0) (1.0 0.0)))
      (`CanvasPanelSlot.SetPosition` _returnvalue_2 (`self.Position`)))))