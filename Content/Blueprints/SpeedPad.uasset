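; SpeedPad is an overlap-triggered pad that temporarily speeds up or slows down a ThirdPersonCharacter.
; On overlap it stores the character, clears its sprinting flag and multiplies its current max walk speed by SpeedMultiplier.
; After a SpeedTime delay it resets the stored character's walk speed to that character's DefaultSpeed, rather than the speed it had on entry.
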(event `self.ReceiveActorBeginOverlap`
  (params (OtherActor :type "Actor Object Reference"))
  (bind _character (`self.Character`))
  ;[1 1 1] SpeedPad Activation (can also decrease the speed)
  (bind _asthird_person_character (cast `/Game/ThirdPersonCPP/Blueprints/ThirdPersonCharacter` OtherActor))
  (bind _output_get (set `self.Character` _asthird_person_character))
  (set `Dev_TemplateCharacter.IsSprinting` false _output_get)
  (bind _charactermovement (`Character.CharacterMovement` _asthird_person_character))
  (set `CharacterMovementComponent.MaxWalkSpeed` (* (`CharacterMovementComponent.MaxWalkSpeed` _charactermovement) (`self.SpeedMultiplier`)) _charactermovement)
  (`KismetSystemLibrary.Delay` (`self.SpeedTime`))
  (set `CharacterMovementComponent.MaxWalkSpeed` (`/Game/ThirdPersonCPP/Blueprints/ThirdPersonCharacter.DefaultSpeed` _character) (`Character.CharacterMovement` _character)))

(fn `UserConstructionScript`)