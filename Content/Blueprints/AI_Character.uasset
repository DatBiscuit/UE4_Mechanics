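; AI_Character is an enemy-style actor that explodes when shot or when the player touches it.
; A hit from a FirstPersonProjectile spawns an explosion particle and sound at its location, then destroys both the actor and the projectile.
; Overlap with the first player character triggers the same effects and destroys only the actor.
; The graph contains no movement, AI or damage logic.
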(event `self.ReceiveHit`
  (params (MyComp :type "PrimitiveComponent Object Reference") (Other :type "Actor Object Reference") (OtherComp :type "PrimitiveComponent Object Reference") (bSelfMoved :type Boolean) (HitLocation :type "Vector Structure") (HitNormal :type "Vector Structure") (NormalImpulse :type "Vector Structure") (Hit :type "HitResult Structure (by ref)"))
  (bind _returnvalue (`self.K2_GetActorLocation`))
  (bind _asfirst_person_projectile (cast `/Game/FirstPersonBP/Blueprints/FirstPersonProjectile` Other))
  (`GameplayStatics.SpawnEmitterAtLocation` "/Game/StarterContent/Particles/P_Explosion.P_Explosion" _returnvalue)
  (`GameplayStatics.SpawnSoundAtLocation` "/Game/StarterContent/Audio/Explosion01.Explosion01" _returnvalue (struct) 1.0 1.0 0.0 null null)
  (`self.K2_DestroyActor`)
  (`self.K2_DestroyActor` _asfirst_person_projectile))

(event `self.ReceiveActorBeginOverlap`
  (params (OtherActor :type "Actor Object Reference"))
  (bind _returnvalue (`self.K2_GetActorLocation`))
  (if (== OtherActor (`GameplayStatics.GetPlayerCharacter` 0))
    (`GameplayStatics.SpawnEmitterAtLocation` "/Game/StarterContent/Particles/P_Explosion.P_Explosion" _returnvalue)
    (`GameplayStatics.SpawnSoundAtLocation` "/Game/StarterContent/Audio/Explosion01.Explosion01" _returnvalue (struct) 1.0 1.0 0.0 null null)
    (`self.K2_DestroyActor`)))

(fn `UserConstructionScript`)