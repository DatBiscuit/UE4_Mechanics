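; CameraRotation is a trigger volume that smoothly rotates the third-person character's follow camera to a set orientation.
; On overlap it casts the other actor to ThirdPersonCharacter, stores its FollowCamera and raises a rotate flag.
; Tick then interpolates the camera's relative rotation toward RotationTarget with RInterpTo, clearing the flag once it matches within a small tolerance.
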(event `self.ReceiveActorBeginOverlap`
  (params (OtherActor :type "Actor Object Reference"))
  ;[1 1 1] Change Rotate Camera to true when collided with volume
  (bind _asthird_person_character (cast `/Game/ThirdPersonCPP/Blueprints/ThirdPersonCharacter` OtherActor))
  (set `self.CharacterCamera` (`Dev_TemplateCharacter.FollowCamera` _asthird_person_character))
  (set `self.RotateCamera` true))

(event `self.ReceiveTick`
  (params (DeltaSeconds :type "Float (single-precision)"))
  (bind _rotationtarget (`self.RotationTarget`))
  (bind _charactercamera (`self.CharacterCamera`))
  ;[1 1 1] Rotate the camera smoothly
  (if (`self.RotateCamera`)
    (`SceneComponent.K2_SetRelativeRotation` _charactercamera (`KismetMathLibrary.RInterpTo` (`SceneComponent.RelativeRotation` _charactercamera) _rotationtarget DeltaSeconds 2.0) false false)
    (if (== (`SceneComponent.RelativeRotation` _charactercamera) _rotationtarget :`ErrorTolerance` 0.01)
      (set `self.RotateCamera` false))))

(fn `UserConstructionScript`)