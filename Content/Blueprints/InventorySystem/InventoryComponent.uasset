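; Inventory component that holds items in a fixed-size slot array, toggles the inventory window and tracks armor.
; Stackable items top up a partial stack found by a macro, recursively re-adding overflow; others take an empty slot.
; The toggle creates or removes a centered widget on the HUD canvas and switches input mode.
; Equipping armor records it by slot and refreshes character stats, while AddToEquipment stores only armor, ignoring its weapon input.
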(event `self.ReceiveBeginPlay`
  (`self.PrepareInventory`))

(fn `AddToEquipment`
  (params (Armor :type "/Game/Blueprints/Data/Armor_Data Structure") (Weapon :type "/Game/Blueprints/Data/Weapon_Data Structure"))
  (`KismetArrayLibrary.Array_Add` (`self.ArmorContent`) Armor))

(fn `AddToInventory`
  (params (ContentToAdd :type "/Game/Blueprints/InventorySystem/SlotStructure Structure"))
  (returns (Success :type Boolean))
  (bind _contenttoadd (`local.ContentToAdd`))
  (if (`.IsStackable_9_F62DB7B94DB3AC76E89B389FD63BE318` (break `/Game/Blueprints/InventorySystem/ItemStructure` (break `/Game/Blueprints/InventorySystem/SlotStructure` ContentToAdd)))
    (bind _stackindex (`self.HasPartialStack` _contenttoadd)
      (:`True`
        (`self.AddToStack` _contenttoadd _stackindex))
      (:`False`
        (`self.CreateStack` _contenttoadd :!label _label)))
    (else
      (goto _label)))
  (return true))

(fn `AddToStack`
  (params (SlotStructure :type "/Game/Blueprints/InventorySystem/SlotStructure Structure") (SlotIndex :type Integer))
  (locals (CurrentQuantity :type Integer))
  (bind (_slotstructure_itemstructure _slotstructure_quantity) (break `/Game/Blueprints/InventorySystem/SlotStructure` (`local.SlotStructure`)))
  (bind _inventory (`self.Inventory`))
  (bind _slotindex (`local.SlotIndex`))
  (bind _slotstructure_itemstructure_2 (break `/Game/Blueprints/InventorySystem/SlotStructure` (`local.SlotStructure`)))
  (bind (_slotstructure_itemstructure_3 _slotstructure_quantity_2) (break `/Game/Blueprints/InventorySystem/SlotStructure` (`local.SlotStructure`)))
  (bind (_name _isstackable _thumbnail _description _isconsumable _maxstacksize) (break `/Game/Blueprints/InventorySystem/ItemStructure` _slotstructure_itemstructure_2))
  (bind _output (`|GetArrayItem` (`self.Inventory`) SlotIndex))
  (bind (_output_itemstructure _output_quantity) (break `/Game/Blueprints/InventorySystem/SlotStructure` (`|GetArrayItem` _inventory _slotindex)))
  (bind _output_get (set `local.CurrentQuantity` (`.Quantity_6_07FA3DDF4CCE1EBADDC2B29E982E8C51` (break `/Game/Blueprints/InventorySystem/SlotStructure` _output))))
  (if (> (+ _output_get (`.Quantity_6_07FA3DDF4CCE1EBADDC2B29E982E8C51` (break `/Game/Blueprints/InventorySystem/SlotStructure` SlotStructure))) (`.MaxStackSize_16_A993FABD4902E212C77BF88833855B62` (break `/Game/Blueprints/InventorySystem/ItemStructure` (break `/Game/Blueprints/InventorySystem/SlotStructure` _output))))
    (`KismetArrayLibrary.Array_Set` (`self.Inventory`) (`local.SlotIndex`) (make `/Game/Blueprints/InventorySystem/SlotStructure` _slotstructure_itemstructure_2 _maxstacksize))
    (`self.AddToInventory` (make `/Game/Blueprints/InventorySystem/SlotStructure` _slotstructure_itemstructure_3 (- _slotstructure_quantity_2 (- _maxstacksize (`local.CurrentQuantity`)))))
    (else
      (`KismetArrayLibrary.Array_Set` _inventory _slotindex (make `/Game/Blueprints/InventorySystem/SlotStructure` _output_itemstructure (+ _output_quantity _slotstructure_quantity)))))
  (return))

(fn `CreateStack`
  (params (ContentToAdd :type "/Game/Blueprints/InventorySystem/SlotStructure Structure"))
  (bind _inventory (`self.Inventory`))
  (`KismetArrayLibrary.Array_Set` _inventory (`KismetArrayLibrary.Array_Find` _inventory (make `/Game/Blueprints/InventorySystem/SlotStructure` (struct :`Name` "NSLOCTEXT(\"[9128BB1746FA0F24CAF76DA1D9271005]\", \"B1F7ED1A438BB4C98C9859AFEBC3B815\", \"None\")" :`IsStackable` true :`Description` "NSLOCTEXT(\"[9128BB1746FA0F24CAF76DA1D9271005]\", \"310EC7EB42385D419D9C5DB2CDA42956\", \"None\")" :`IsConsumable` true :`MaxStackSize` 4))) ContentToAdd))

(fn `EquipArmor`
  (params (ArmorSlot :type "/Game/Blueprints/Data/ArmorType Enum" :default "NewEnumerator0") (Armor :type "/Game/Blueprints/Data/Armor_Data Structure"))
  (`BlueprintMapLibrary.Map_Add` (`self.EquippedArmor`) ArmorSlot Armor)
  (bind _asthird_person_character (cast `/Game/ThirdPersonCPP/Blueprints/ThirdPersonCharacter` (`GameplayStatics.GetPlayerCharacter` 0)))
  (`/Game/ThirdPersonCPP/Blueprints/ThirdPersonCharacter.RefreshStats` _asthird_person_character))

(fn `PrepareInventory`
  (`KismetArrayLibrary.Array_Resize` (`self.Inventory`) (`self.NumberOfSlots`)))

(fn `ToggleInventory`
  (`self.InventoryWindow`
    (:`then`
      ;[1 1 1] Turn off inventory
      (`Widget.RemoveFromParent` (`self.InventoryWindow`))
      (set `self.InventoryWindow` null)
      (`WidgetBlueprintLibrary.SetInputMode_GameOnly` (`GameplayStatics.GetPlayerController` 0)))
    (:`else`
      (bind _returnvalue (`|CreateWidget` "/Game/Blueprints/InventorySystem/InventoryWindow.InventoryWindow_C" null self))
      (set `self.InventoryWindow` _returnvalue)
      (bind _asmy_player_controller (cast `/Game/Blueprints/MyPlayerController` (`GameplayStatics.GetPlayerController` 0)))
      (bind _returnvalue_2 (`CanvasPanel.AddChildToCanvas` (`/Game/Blueprints/HUD.HudCanvas` (`/Game/Blueprints/MyPlayerController.Hud Widget` _asmy_player_controller)) (`self.InventoryWindow`)))
      (`CanvasPanelSlot.SetAutoSize` _returnvalue_2 true)
      (`CanvasPanelSlot.SetAlignment` _returnvalue_2 (0.5 0.5))
      (`CanvasPanelSlot.SetAnchors` _returnvalue_2 (make `Anchors` (0.5 0.5) (0.5 0.5)))
      (`CanvasPanelSlot.SetPosition` _returnvalue_2 (`self.Position`))
      (`WidgetBlueprintLibrary.SetInputMode_UIOnlyEx` (`GameplayStatics.GetPlayerController` 0) (`self.InventoryWindow`) "LockAlways"))))